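; BP_SecurityCamController is the AI controller for a security camera that raises an alarm when it detects the player.
; On an AI Perception update for a ThirdPersonCharacter, it plays the Red_Alert sound at the controlled pawn's location and adds the UMG_Detected widget to the viewport.
; The PlayerDetected flag makes this a one-shot alarm, as nothing here resets it.
; The stimulus's sensed state is not checked.
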(event `self.AIPerception.OnTargetPerceptionUpdated`
  (params (Actor :type "Actor Object Reference") (Stimulus :type "AIStimulus Structure"))
  (if (not (`self.playerDetected`))
    (cast `/Game/ThirdPersonBP/Blueprints/ThirdPersonCharacter` Actor)
    (set `self.playerDetected` true)
    (`GameplayStatics.PlaySoundAtLocation` "/Game/SourceContent/Red_Alert.Red_Alert" (`self.K2_GetActorLocation` (`self.K2_GetPawn`)) (struct) 1.0 1.0 0.0 null null null)
    (bind _returnvalue (`|CreateWidget` "/Game/UMG/UMG_Detected.UMG_Detected_C" (`GameplayStatics.GetPlayerController` 0)))
    (`UserWidget.AddToViewport` _returnvalue 0)))

(fn `UserConstructionScript`)