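; BP_LockedDoor is a door actor that slides away from its starting position when its OpenDoor event fires; it contains no lock check.
; BeginPlay caches the actor location, and a FlipFlop alternates the sign of the travel scale on each OpenDoor call.
; OpenTimeline then plays, setting the actor's relative location each update to the cached location plus the scaled Open track, without sweeping.
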(event `self.ReceiveBeginPlay`
  (set `self.StartingLocation` (`self.K2_GetActorLocation`)))

(event `self.OpenDoor`
  (`/Engine/EditorBlueprintResources/StandardMacros.FlipFlop`
    (:`A`
      (set `self.Scale` -200.0)
      (bind (_direction _open) (`Timeline|OpenTimeline` :!label _label)
        (:`Update`
          (`self.K2_SetActorRelativeLocation` (+ (* _open (`self.Scale`)) (`self.StartingLocation`))))))
    (:`B`
      (set `self.Scale` 200.0)
      (goto _label))))

(fn `UserConstructionScript`)